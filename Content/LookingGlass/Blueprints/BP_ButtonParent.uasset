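; BP_ButtonParent is a base Blueprint for buttons in the LookingGlass content, providing a color toggle on a static mesh.
; On BeginPlay it creates a dynamic material instance from the mesh's first material slot and enables input from the first player controller.
; SetColor turns the material's color parameter red and UnSetColor turns it green.
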(event `self.ReceiveBeginPlay`
  (bind _staticmesh (`self.StaticMesh`))
  (bind _returnvalue (`PrimitiveComponent.CreateDynamicMaterialInstance` _staticmesh 0 (`PrimitiveComponent.GetMaterial` _staticmesh 0) "None"))
  (set `self.DynamicMaterail` _returnvalue)
  (`self.EnableInput` (`GameplayStatics.GetPlayerController` 0)))

(fn `SetColor`
  (`MaterialInstanceDynamic.SetVectorParameterValue` (`self.DynamicMaterail`) (`self.ColorParameter`) (make `LinearColor` 1.0)))

(fn `UnSetColor`
  (`MaterialInstanceDynamic.SetVectorParameterValue` (`self.DynamicMaterail`) (`self.ColorParameter`) (make `LinearColor` 0.0 1.0)))

(fn `UserConstructionScript`)